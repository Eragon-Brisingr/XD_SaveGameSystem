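; Example game mode that hooks an auto save/load system into the level lifecycle and player spawning.
; It initializes the system on BeginPlay and shuts it down on EndPlay.
; SpawnDefaultPawnFor first tries to load a saved player for the controller, falling back to the parent's default spawn.
; Either pawn is then registered with the system for auto-saving.
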(event EventBeginPlay
  (Class|XDSaveGameFunctionLibrary|InitAutoSaveLoadSystem self))

(event EventTick
  (params (DeltaSeconds :type Float%20%28single-precision%29)))

(event EventEndPlay
  (params (EndPlayReason :type EEndPlayReason%20Enum :default "Destroyed"))
  (Class|XDSaveGameFunctionLibrary|ShutDownAutoSaveLoadSystem self))

(fn ConstructionScript)

(fn SpawnDefaultPawnfor
  (params (NewPlayer :type Controller%20Object%20Reference) (StartSpot :type Actor%20Object%20Reference))
  (bind _asplayer_controller (Utilities|Casting|CastToPlayerController NewPlayer)
    (:then
      (bind _returnvalue (Class|XDSaveGameFunctionLibrary|TryLoadPlayer _asplayer_controller))
      (Utilities|IsValid _returnvalue
        (:Is%20Valid
          (Class|XDSaveGameFunctionLibrary|RegisterAutoSavePlayer _returnvalue)
          (return _returnvalue))
        (:Is%20Not%20Valid
          _)))
    (:CastFailed
      _))
  (bind _returnvalue_2 (|CallParentFunction NewPlayer StartSpot))
  (Class|XDSaveGameFunctionLibrary|RegisterAutoSavePlayer _returnvalue_2)
  (return _returnvalue_2))