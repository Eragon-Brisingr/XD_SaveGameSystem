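; Example actor that demonstrates the XD save system's lifecycle hooks and opts in to saving.
; NeedSave always returns true.
; The game-init, post-load and pre-save events each print the actor's display name with a Chinese label for that phase.
; It holds no state or gameplay logic of its own.
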(event EventBeginPlay)

(event Collision|EventActorBeginOverlap
  (params (OtherActor :type Actor%20Object%20Reference)))

(event EventTick
  (params (DeltaSeconds :type Float%20%28single-precision%29)))

(event EventWhenGameInit
  (Development|PrintString (Utilities|String|Append (Utilities|GetDisplayName self) " 游戏初始化")))

(event EventWhenPostLoad
  (Development|PrintString (Utilities|String|Append (Utilities|GetDisplayName self) " 游戏读取")))

(event EventWhenPreSave
  (Development|PrintString (Utilities|String|Append (Utilities|GetDisplayName self) " 游戏存档")))

(fn ConstructionScript)

(fn NeedSave
  (return true))